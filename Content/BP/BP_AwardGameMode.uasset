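; Game mode that runs stage-based play for the BP_Award pawn, handling respawns, stage streaming and the play UI.
; It rebinds to the pawn's OnDestroyed, spawning and possessing a new BP_Award at the player start each time.
; Stages are blocking-loaded streamed sublevels; NextStage unloads the current one and increments the number in its name.
; After each load the pawn is moved to the player start, since sublevel placement leaves it at a default position.
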(event Custom|RespawnEvent
  (Game|AssignOnDestroyed (Game|Player|GetPlayerPawn 0) (delegate Custom|RepawnAward)))

(event Custom|RepawnAward
  (params (DestroyedActor :type Actor%20Object%20Reference))
  (bind _returnvalue (Game|SpawnActorfromClass "/Game/BP/BP_Award.BP_Award_C" (Transformation|GetActorTransform (Class|GameModeBase|FindPlayerStart)) "Undefined" 0 0))
  (Pawn|Possess (Game|GetPlayerController 0) _returnvalue)
  (CallFunction|RespawnEvent))

(event Custom|LoadStage
  (Game|LoadStreamLevel(byName) (Variables|Default|GetStageName) true true)
  (CallFunction|SetAwardTransform))

(event Custom|NextStage
  (Game|UnloadStreamLevel(byName) (Variables|Default|GetStageName) true)
  (bind _output_get (Variables|Default|SetStageName (Utilities|String|StringToName (Utilities|String|Append (Utilities|String|Left (Utilities|String|ToString(Name) (Variables|Default|GetStageName)) 5) (Utilities|String|ToString(Integer) (+ (Math|Conversions|ToInteger(Byte) (Utilities|String|RightChop (Utilities|String|ToString(Name) (Variables|Default|GetStageName)) 5)) 1))))))
  (Game|LoadStreamLevel(byName) _output_get true true)
  (CallFunction|SetAwardTransform))

(event Custom|CreateUI
  (bind _returnvalue (UserInterface|CreateWidget "/Game/UI/W_Play.W_Play_C"))
  (UserInterface|Viewport|AddtoViewport _returnvalue 0))

(event EventBeginPlay
  (CallFunction|RespawnEvent)
  (CallFunction|LoadStage)
  (CallFunction|CreateUI))

(event EventTick
  (params (DeltaSeconds :type Float%20%28single-precision%29)))

(fn ConstructionScript)

(fn SetAwardTransform
  ;[1 1 1] サブレベルで置いた時はデフォ位置になるのでプレイヤーの位置をセットし直す
  (Transformation|SetActorTransform (Game|Player|GetPlayerPawn 0) (Transformation|GetActorTransform (Class|GameModeBase|FindPlayerStart))))