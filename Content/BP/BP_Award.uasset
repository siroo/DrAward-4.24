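; BP_Award is a character with a head light and point light that handles damage death and lives.
; On BeginPlay it turns both lights red if the level is "End" and the game instance is not cleared.
; The first damage disables movement and ragdolls the mesh.
; It then either spends a life from AwardGameInstance and expires after a short lifespan, or opens the End level after a delay when none remain.
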(event EventBeginPlay
  (bind _returnvalue (Game|GetCurrentLevelName true))
  (bind _asaward_game_instance (Utilities|Casting|CastToAwardGameInstance (Game|GetGameInstance)))
  (if (and (Utilities|Enum|Equal(Enum) _returnvalue "End") (not (Variables|/Game/BP/AwardGAmeInstance.AwardGameInstance_C|GetIsClear _asaward_game_instance)))
    (Rendering|Components|Light|SetLightColor (Variables|Default|GetHeadLight) "(R=1.000000,G=0.000000,B=0.000000,A=1.000000)" true)))

(event Collision|EventActorBeginOverlap
  (params (OtherActor :type Actor%20Object%20Reference)))

(event Game|Damage|EventAnyDamage
  (params (Damage :type Float%20%28single-precision%29) (DamageType :type Damage%20Type%20Object%20Reference) (InstigatedBy :type Controller%20Object%20Reference) (DamageCauser :type Actor%20Object%20Reference))
  (bind _returnvalue (Game|GetGameInstance))
  (bind _mesh (Variables|Character|GetMesh))
  (bind _asaward_game_instance (Utilities|Casting|CastToAwardGameInstance _returnvalue))
  (Utilities|FlowControl|DoOnce false
    (:Completed
      (Utilities|FlowControl|Sequence
        (:then_0
          (Pawn|Components|CharacterMovement|DisableMovement (Variables|Character|GetCharacterMovement))
          (Collision|SetCollisionProfileName _mesh "Ragdoll" :!class /Script/Engine.PrimitiveComponent)
          (Physics|SetSimulatePhysics _mesh true))
        (:then_1
          (if (> (Variables|/Game/BP/AwardGAmeInstance.AwardGameInstance_C|GetLife _asaward_game_instance) 0)
            (Variables|/Game/BP/AwardGAmeInstance.AwardGameInstance_C|SetLife _asaward_game_instance (- (Variables|/Game/BP/AwardGAmeInstance.AwardGameInstance_C|GetLife _asaward_game_instance) 1))
            (Actor|SetLifeSpan 3.0)
            (else
              (Utilities|FlowControl|Delay 3.0)
              (Game|OpenLevel(byName) "End"))))))))

(fn ConstructionScript)